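; Actor component that detects the puzzle interactable the camera is looking at.
; Every tick it runs a thin, short-range sphere trace on the Visibility channel along the camera's forward vector.
; A hit actor implementing I_Puzzle receives SelectedMessage(true) and is stored as CurrentInteractable.
; Otherwise CurrentInteractable is cleared, with no deselect message sent to the previous actor.
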(event `self.ReceiveTick`
  (params (DeltaSeconds :type "Float (single-precision)"))
  (`self.Check`))

(event `Check`
  (bind _camera (`self.Camera`))
  (bind _returnvalue (`SceneComponent.K2_GetComponentLocation` _camera))
  (bind _outhit (`KismetSystemLibrary.SphereTraceSingle` _returnvalue (+ _returnvalue (* (`SceneComponent.GetForwardVector` _camera) 240.0)) 1.0 "TraceTypeQuery1"))
  (bind (_bblockinghit _binitialoverlap _time _distance _location _impactpoint _normal _impactnormal _physmat _hitactor) (`GameplayStatics.BreakHitResult` _outhit))
  (if (`KismetSystemLibrary.DoesImplementInterface` _hitactor "/Game/Blueprints/Interfaces/I_Puzzle.I_Puzzle_C")
    (message `/Game/Blueprints/Interfaces/I_Puzzle.Selected` _hitactor true)
    (set `self.CurrentInteractable` _hitactor)
    (else
      (set `self.CurrentInteractable` null))))