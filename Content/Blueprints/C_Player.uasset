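; First-person player character for a puzzle game, with Enhanced Input movement, look, jump, sprint and crouch, plus a crosshair HUD.
; An interactable-check component on the camera supplies the Interact target, while held objects lerp by timeline to an attach point until dropped.
; A timeline drives speed-scaled head wobble, and a sphere trace gates standing up.
; Destruction notifies GM_Puzzle, and cheat inputs teleport to eight level locations.
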(event `self.ReceiveBeginPlay`
  (`self.Setup Input`)
  (`self.init HUD`)
  (`self.HeadWobble`)
  (`self.Setup Camera`)
  (`self.Setup Variables`))

(event `init HUD`
  ;[1 1 1] HUD
  (bind _returnvalue (`|GenericCreateObject` "/Game/UI/UW_Crosshair.UW_Crosshair_C"))
  (bind _output_get (set `self.HUD` _returnvalue))
  (`UserWidget.AddToViewport` _output_get 0))

(event `Setup Variables`
  ;[1 1 1] Setup Variables
)

(event `HeadWobble`
  (bind _charactermovement (`self.CharacterMovement`))
  ;[1 1 1] HeadWobble
  (`TimelineComponent.SetPlayRate` (`self.HeadMovement`) (`self.HeadWobbleRate`))
  (bind (_direction _alpha) (`Timeline|HeadMovement`)
    (:`Update`
      (`SceneComponent.K2_SetRelativeLocation` (`self.Camera`) (`KismetMathLibrary.MakeVector` 0.0 0.0 (* _alpha (`self.HeadWobbleAmount`) (`KismetMathLibrary.MapRangeClamped` (`KismetMathLibrary.VSizeXY` (`MovementComponent.Velocity` _charactermovement)) 0.0 (`CharacterMovementComponent.MaxWalkSpeed` _charactermovement) 0.3 5.0))) false true))))

(event `EnhancedInput|/Game/Inputs/IA_Crouch`
  (params (ActionValue :type Boolean) (ElapsedSeconds :type "Float (double-precision)") (TriggeredSeconds :type "Float (double-precision)") (InputAction :type "InputAction Object Reference" :default "/Game/Inputs/IA_Crouch.IA_Crouch"))
  (bind _returnvalue (`SceneComponent.K2_GetComponentLocation` (`self.Scene`)))
  (bind (_x _y _z) (`KismetMathLibrary.BreakVector3f` _returnvalue))
  ;[1 1 1] Crouch
  (:`Started`
    (if (`NavMovementComponent.IsCrouching` (`self.CharacterMovement`))
      (bind (_outhits _returnvalue_2) (`KismetSystemLibrary.SphereTraceMulti` _returnvalue (`KismetMathLibrary.MakeVector` _x _y (+ _z (`CharacterMovementComponent.CrouchedHalfHeight` (`self.CharacterMovement`)))) (`CapsuleComponent.GetUnscaledCapsuleRadius` (`self.CapsuleComponent`)) "TraceTypeQuery1"))
      (if (not _returnvalue_2)
        (`self.UnCrouch`)
        (`SceneComponent.K2_AddRelativeLocation` (`self.Scene`) (0.0 0.0 30.0) false false))
      (else
        (`self.Crouch`)
        (`SceneComponent.K2_AddRelativeLocation` (`self.Scene`) (0.0 0.0 -30.0) false false)))))

(event `EnhancedInput|/Game/Inputs/IA_Sprint`
  (params (ActionValue :type Boolean) (ElapsedSeconds :type "Float (double-precision)") (TriggeredSeconds :type "Float (double-precision)") (InputAction :type "InputAction Object Reference" :default "/Game/Inputs/IA_Sprint.IA_Sprint"))
  ;[1 1 1] Sprint
  (:`Started`
    (set `CharacterMovementComponent.MaxWalkSpeed` (* (`CharacterMovementComponent.MaxWalkSpeed` (`self.CharacterMovement`)) (`self.SprintMultiplier`)) (`self.CharacterMovement`)))
  (:`Completed`
    (set `CharacterMovementComponent.MaxWalkSpeed` (/ (`CharacterMovementComponent.MaxWalkSpeed` (`self.CharacterMovement`)) (`self.SprintMultiplier`)) (`self.CharacterMovement`))))

(event `self.ReceiveDestroyed`
  ;[1 1 1] Playerdeath
  (bind _asgm_puzzle (cast `/Game/Blueprints/GM_Puzzle` (`GameplayStatics.GetGameMode`)))
  (`/Game/Blueprints/GM_Puzzle.PlayerDied` _asgm_puzzle))

(event `Pickup Object`
  (params (`Object to Pickup` :type "/Game/Blueprints/A_Pickupable Object Reference"))
  ;[1 1 1] Pickup Object
  (bind _output_get (set `self.HandSlot` `Object to Pickup`))
  (set `self.PickupOrigin` (`SceneComponent.K2_GetComponentLocation` (`Actor.RootComponent` _output_get)))
  (bind (_direction _alpha) (`Timeline|Pickup` :!via `PlayFromStart` :!label _label)
    (:`Update`
      (`self.K2_SetActorLocation` (`self.HandSlot`) (`KismetMathLibrary.VLerp` (`self.PickupOrigin`) (`SceneComponent.K2_GetComponentLocation` (`self.PickupPoint`)) _alpha) false false))
    (:`Finished`
      (`self.K2_AttachToComponent` (`self.HandSlot`) (`self.PickupPoint`) "None" "SnapToTarget" "KeepRelative" "KeepRelative" true))))

(event `InterruptPickup`
  ;[1 1 1] Pickup Object
  (goto _label :!via `Stop`))

(event `Drop Object`
  (bind _handslot (`self.HandSlot`))
  (`/Engine/EditorBlueprintResources/StandardMacros.IsValid` _handslot
    (:`Is Valid`
      (`self.InterruptPickup`)
      (`self.K2_DetachFromActor` _handslot "KeepWorld" "KeepWorld" "KeepRelative")
      (`/Game/Blueprints/A_Pickupable.Dropped` (`self.HandSlot`) (`KismetMathLibrary.GetForwardVector` (`self.GetControlRotation`)))
      (set `self.HandSlot` null))))

(event `Setup Input`
  ;[1 1 1] Setup Input
  (`EnhancedInputSubsystemInterface.AddMappingContext` (pcsubsystem `EnhancedInputLocalPlayerSubsystem` (`GameplayStatics.GetPlayerController` 0)) "/Game/Inputs/IMC_Player.IMC_Player" 0 (struct)))

(event `EnhancedInput|/Game/Inputs/IA_Jump`
  (params (ActionValue :type Boolean) (ElapsedSeconds :type "Float (double-precision)") (TriggeredSeconds :type "Float (double-precision)") (InputAction :type "InputAction Object Reference" :default "/Game/Inputs/IA_Jump.IA_Jump"))
  (:`Started`
    (`self.Jump`)))

(event `EnhancedInput|/Game/Inputs/IA_Move`
  (params (ActionValue :type "Vector2D Structure") (ElapsedSeconds :type "Float (double-precision)") (TriggeredSeconds :type "Float (double-precision)") (InputAction :type "InputAction Object Reference" :default "/Game/Inputs/IA_Move.IA_Move"))
  (bind (_returnvalue_roll _returnvalue_pitch _returnvalue_yaw) (`KismetMathLibrary.BreakRotator` (`self.GetControlRotation`)))
  (bind (_returnvalue_roll_2 _returnvalue_pitch_2 _returnvalue_yaw_2) (`KismetMathLibrary.BreakRotator` (`self.GetControlRotation`)))
  (:`Triggered`
    ;[1 1 1] Move Forward/Backwards
    (`self.AddMovementInput` (`KismetMathLibrary.GetForwardVector` (`KismetMathLibrary.MakeRotator` 0.0 0.0 _returnvalue_yaw)) ActionValue_Y)
    ;[1 1 1] Move Right/Left
    (`self.AddMovementInput` (`KismetMathLibrary.GetRightVector` (`KismetMathLibrary.MakeRotator` 0.0 0.0 _returnvalue_yaw_2)) ActionValue_X)))

(event `EnhancedInput|/Game/Inputs/IA_Look`
  (params (ActionValue :type "Vector2D Structure") (ElapsedSeconds :type "Float (double-precision)") (TriggeredSeconds :type "Float (double-precision)") (InputAction :type "InputAction Object Reference" :default "/Game/Inputs/IA_Look.IA_Look"))
  (:`Triggered`
    ;[1 1 1] Look
    (`self.AddControllerYawInput` (* ActionValue_X (`self.LookSensitivity`)))
    (`self.AddControllerPitchInput` (* (* ActionValue_Y (`self.LookSensitivity`)) (`KismetMathLibrary.SelectInt` -1 1 (`self.Invert Y-Axis`))))))

(event `EnhancedInput|/Game/Inputs/IA_Interact`
  (params (ActionValue :type Boolean) (ElapsedSeconds :type "Float (double-precision)") (TriggeredSeconds :type "Float (double-precision)") (InputAction :type "InputAction Object Reference" :default "/Game/Inputs/IA_Interact.IA_Interact"))
  (bind _currentinteractable (`/Game/Blueprints/Components/AC_CheckForInteractable.CurrentInteractable` (`self.CheckForInteractable`)))
  (:`Started`
    ;[1 1 1] Interact
    (`/Engine/EditorBlueprintResources/StandardMacros.IsValid` (`self.HandSlot`)
      (:`Is Valid`
        (`self.Drop Object`))
      (:`Is Not Valid`
        (`/Engine/EditorBlueprintResources/StandardMacros.IsValid` _currentinteractable
          (:`Is Valid`
            (message `/Game/Blueprints/Interfaces/I_Puzzle.Interact` _currentinteractable self)))))))

(event `self.ReceivePossessed`
  (params (NewController :type "Controller Object Reference"))
  ;[1 1 1] Player Inputs Hinzufügen
  (`self.Setup Input`))

(event `self.ReceiveUnpossessed`
  (params (OldController :type "Controller Object Reference"))
  ;[1 1 1] Player Inputs leeren
  (`EnhancedInputSubsystemInterface.RemoveMappingContext` (pcsubsystem `EnhancedInputLocalPlayerSubsystem` (`GameplayStatics.GetPlayerController` 0)) "/Game/Inputs/IMC_Player.IMC_Player" (struct)))

(event `EnhancedInput|/Game/Inputs/Tps/Lv_1`
  (params (ActionValue :type Boolean) (ElapsedSeconds :type "Float (double-precision)") (TriggeredSeconds :type "Float (double-precision)") (InputAction :type "InputAction Object Reference" :default "/Game/Inputs/Tps/Lv_1.Lv_1"))
  ;[1 1 1] Cheats
  (:`Started`
    ;;[1 1 1] Lv1
    (`SceneComponent.K2_SetWorldLocation` (`self.CapsuleComponent`) (-9260.0 1410.0 1872.0) false false)))

(event `EnhancedInput|/Game/Inputs/Tps/Lv_5`
  (params (ActionValue :type Boolean) (ElapsedSeconds :type "Float (double-precision)") (TriggeredSeconds :type "Float (double-precision)") (InputAction :type "InputAction Object Reference" :default "/Game/Inputs/Tps/Lv_5.Lv_5"))
  ;[1 1 1] Cheats
  (:`Started`
    ;;[1 1 1] Lv 5
    (`SceneComponent.K2_SetWorldLocation` (`self.CapsuleComponent`) (-4620.0 -2850.0 872.0) false false)))

(event `EnhancedInput|/Game/Inputs/Tps/Lv_2`
  (params (ActionValue :type Boolean) (ElapsedSeconds :type "Float (double-precision)") (TriggeredSeconds :type "Float (double-precision)") (InputAction :type "InputAction Object Reference" :default "/Game/Inputs/Tps/Lv_2.Lv_2"))
  ;[1 1 1] Cheats
  (:`Started`
    ;;[1 1 1] Lv2
    (`SceneComponent.K2_SetWorldLocation` (`self.CapsuleComponent`) (-8020.0 -590.0 1392.0) false false)))

(event `EnhancedInput|/Game/Inputs/Tps/Lv_6`
  (params (ActionValue :type Boolean) (ElapsedSeconds :type "Float (double-precision)") (TriggeredSeconds :type "Float (double-precision)") (InputAction :type "InputAction Object Reference" :default "/Game/Inputs/Tps/Lv_6.Lv_6"))
  ;[1 1 1] Cheats
  (:`Started`
    ;;[1 1 1] Lv6
    (`SceneComponent.K2_SetWorldLocation` (`self.CapsuleComponent`) (-2000.0 -2850.0 872.0) false false)))

(event `EnhancedInput|/Game/Inputs/Tps/Lv_7`
  (params (ActionValue :type Boolean) (ElapsedSeconds :type "Float (double-precision)") (TriggeredSeconds :type "Float (double-precision)") (InputAction :type "InputAction Object Reference" :default "/Game/Inputs/Tps/Lv_7.Lv_7"))
  ;[1 1 1] Cheats
  (:`Started`
    ;;[1 1 1] Lv7
    (`SceneComponent.K2_SetWorldLocation` (`self.CapsuleComponent`) (-900.0 -690.0 872.0) false false)))

(event `EnhancedInput|/Game/Inputs/Tps/Lv_3`
  (params (ActionValue :type Boolean) (ElapsedSeconds :type "Float (double-precision)") (TriggeredSeconds :type "Float (double-precision)") (InputAction :type "InputAction Object Reference" :default "/Game/Inputs/Tps/Lv_3.Lv_3"))
  ;[1 1 1] Cheats
  (:`Started`
    ;;[1 1 1] Lv3
    (`SceneComponent.K2_SetWorldLocation` (`self.CapsuleComponent`) (-8020.0 -2150.0 1392.0) false false)))

(event `EnhancedInput|/Game/Inputs/Tps/Lv_8`
  (params (ActionValue :type Boolean) (ElapsedSeconds :type "Float (double-precision)") (TriggeredSeconds :type "Float (double-precision)") (InputAction :type "InputAction Object Reference" :default "/Game/Inputs/Tps/Lv_8.Lv_8"))
  ;[1 1 1] Cheats
  (:`Started`
    ;;[1 1 1] Lv8
    (`SceneComponent.K2_SetWorldLocation` (`self.CapsuleComponent`) (-900.0 1550.0 872.0) false false)))

(event `EnhancedInput|/Game/Inputs/Tps/Lv_4`
  (params (ActionValue :type Boolean) (ElapsedSeconds :type "Float (double-precision)") (TriggeredSeconds :type "Float (double-precision)") (InputAction :type "InputAction Object Reference" :default "/Game/Inputs/Tps/Lv_4.Lv_4"))
  ;[1 1 1] Cheats
  (:`Started`
    ;;[1 1 1] Lv4
    (`SceneComponent.K2_SetWorldLocation` (`self.CapsuleComponent`) (-8020.0 -2850.0 952.0) false false)))

(fn `Setup Camera`
  (bind _returnvalue (`GameplayStatics.GetPlayerCameraManager` 0))
  (set `PlayerCameraManager.ViewPitchMin` -70.0 _returnvalue)
  (set `PlayerCameraManager.ViewPitchMax` 80.0 _returnvalue))

(fn `UserConstructionScript`
  (bind _returnvalue (`AddComponent|NODE_AddAC_CheckForInteractable-0` :`Camera` (`self.Camera`)))
  (set `self.CheckForInteractable` _returnvalue))