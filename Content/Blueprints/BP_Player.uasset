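; First-person player character Blueprint that handles movement, jumping and mouse-look, and shows a crosshair HUD.
; BeginPlay registers the Enhanced Input mapping context, creates the crosshair widget, starts the head bob and limits camera pitch.
; Movement follows control yaw, while look input applies sensitivity and optional Y-axis inversion.
; A timeline drives camera height for head bob, scaled by horizontal speed so a subtle sway remains when idle.
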(event `self.ReceiveBeginPlay`
  (`self.Setup Input`)
  (`self.init HUD`)
  (`self.HeadWobble`)
  (`self.Setup Camera`))

(event `init HUD`
  ;[1 1 1] HUD
  (bind _returnvalue (`|GenericCreateObject` "/Game/UI/UW_Crosshair.UW_Crosshair_C"))
  (bind _output_get (set `self.HUD` _returnvalue))
  (`UserWidget.AddToViewport` _output_get 0))

(event `HeadWobble`
  (bind _charactermovement (`self.CharacterMovement`))
  ;[1 1 1] HeadWobble
  (`TimelineComponent.SetPlayRate` (`self.HeadMovement`) (`self.HeadWobbleRate`))
  (bind (_direction _alpha) (`Timeline|HeadMovement`)
    (:`Update`
      (`SceneComponent.K2_SetRelativeLocation` (`self.Camera`) (`KismetMathLibrary.MakeVector` 0.0 0.0 (* _alpha (`self.HeadWobbleAmount`) (`KismetMathLibrary.MapRangeClamped` (`KismetMathLibrary.VSizeXY` (`MovementComponent.Velocity` _charactermovement)) 0.0 (`CharacterMovementComponent.MaxWalkSpeed` _charactermovement) 0.3 5.0))) false true))))

(event `Setup Input`
  ;[1 1 1] Setup Input
  (`EnhancedInputSubsystemInterface.AddMappingContext` (pcsubsystem `EnhancedInputLocalPlayerSubsystem` (`GameplayStatics.GetPlayerController` 0)) "/Game/Inputs/IMC_Player.IMC_Player" 0 (struct)))

(event `EnhancedInput|/Game/Inputs/IA_Jump`
  (params (ActionValue :type Boolean) (ElapsedSeconds :type "Float (double-precision)") (TriggeredSeconds :type "Float (double-precision)") (InputAction :type "InputAction Object Reference" :default "/Game/Inputs/IA_Jump.IA_Jump"))
  (:`Started`
    (`self.Jump`)))

(event `EnhancedInput|/Game/Inputs/IA_Move`
  (params (ActionValue :type "Vector2D Structure") (ElapsedSeconds :type "Float (double-precision)") (TriggeredSeconds :type "Float (double-precision)") (InputAction :type "InputAction Object Reference" :default "/Game/Inputs/IA_Move.IA_Move"))
  (bind (_returnvalue_roll _returnvalue_pitch _returnvalue_yaw) (`KismetMathLibrary.BreakRotator` (`self.GetControlRotation`)))
  (bind (_returnvalue_roll_2 _returnvalue_pitch_2 _returnvalue_yaw_2) (`KismetMathLibrary.BreakRotator` (`self.GetControlRotation`)))
  (:`Triggered`
    ;[1 1 1] Move Forward/Backwards
    (`self.AddMovementInput` (`KismetMathLibrary.GetForwardVector` (`KismetMathLibrary.MakeRotator` 0.0 0.0 _returnvalue_yaw)) ActionValue_Y)
    ;[1 1 1] Move Right/Left
    (`self.AddMovementInput` (`KismetMathLibrary.GetRightVector` (`KismetMathLibrary.MakeRotator` 0.0 0.0 _returnvalue_yaw_2)) ActionValue_X)))

(event `EnhancedInput|/Game/Inputs/IA_Look`
  (params (ActionValue :type "Vector2D Structure") (ElapsedSeconds :type "Float (double-precision)") (TriggeredSeconds :type "Float (double-precision)") (InputAction :type "InputAction Object Reference" :default "/Game/Inputs/IA_Look.IA_Look"))
  (:`Triggered`
    ;[1 1 1] Look
    (`self.AddControllerYawInput` (* ActionValue_X (`self.LookSensitivity`)))
    (`self.AddControllerPitchInput` (* (* ActionValue_Y (`self.LookSensitivity`)) (`KismetMathLibrary.SelectInt` -1 1 (`self.Invert Y-Axis`))))))

(fn `Setup Camera`
  (bind _returnvalue (`GameplayStatics.GetPlayerCameraManager` 0))
  (set `PlayerCameraManager.ViewPitchMin` -70.0 _returnvalue)
  (set `PlayerCameraManager.ViewPitchMax` 80.0 _returnvalue))

(fn `UserConstructionScript`)